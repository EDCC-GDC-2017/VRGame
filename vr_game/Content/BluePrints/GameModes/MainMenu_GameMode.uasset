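; Main menu game mode that creates and switches between the main menu and server browser screens.
; On BeginPlay it adds both widgets to the viewport, passes itself to each as parent, and starts with the server browser hidden.
; Two functions, go to main and go to server browser, swap the screens by toggling visibility rather than recreating the widgets.
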(event `self.ReceiveBeginPlay`
  (bind _returnvalue (`|CreateWidget` "/Game/Widgets/Main_menu/BP_Main_Menu.BP_Main_Menu_C"))
  (set `self.Main_Menu_Widget` _returnvalue)
  (`/Game/Widgets/Main_menu/BP_Main_Menu.Set Parent` _returnvalue self)
  (`UserWidget.AddToViewport` _returnvalue 0)
  (bind _returnvalue_2 (`|CreateWidget` "/Game/Widgets/Main_menu/BP_Server_Browser.BP_Server_Browser_C"))
  (set `self.ServerBrower` _returnvalue_2)
  (`/Game/Widgets/Main_menu/BP_Server_Browser.Set Parent` _returnvalue_2 self)
  (`UserWidget.AddToViewport` _returnvalue_2 0)
  (`Widget.SetVisibility` (`self.ServerBrower`) "Hidden"))

(fn `go to main`
  (`self.Return to main`))

(fn `go to server browser`
  (`self.Got to server browser`))

(fn `UserConstructionScript`)
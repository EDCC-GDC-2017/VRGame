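; BP_VR_HUD is a HUD Blueprint that draws the main player's health as a red bar in the top-left of the screen.
; On each DrawHUD event it casts player character 0 to BP_MainPlayer and scales the bar width by Health against a fixed maximum of 200.
; Position and size scale from a 1920x1080 reference layout to the current screen size, with no clamping on the health ratio.
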(event `self.ReceiveDrawHUD`
  (params (SizeX :type Integer) (SizeY :type Integer))
  (bind _asbp_main_player (cast `/Game/BluePrints/BP_MainPlayer` (`GameplayStatics.GetPlayerCharacter` 0)))
  (`self.DrawRect` (struct :`R` 1.0 :`A` 1.0) (* (/ 20.0 1920.0) (`KismetMathLibrary.Conv_IntToDouble` SizeX)) (* (/ 20.0 1080.0) (`KismetMathLibrary.Conv_IntToDouble` SizeY)) (* (/ (`MainPlayer.health` _asbp_main_player) 200.0) (* (`KismetMathLibrary.Conv_IntToDouble` SizeX) (/ 1000.0 1920.0))) (* (`KismetMathLibrary.Conv_IntToDouble` SizeY) (/ 100.0 1080.0))))

(event `self.ReceiveTick`
  (params (DeltaSeconds :type "Float (single-precision)")))

(fn `UserConstructionScript`)